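; BP_Road is a road floor chunk for a chicken-crossing game that builds itself on BeginPlay.
; It spawns left, center and right floors, with only the center set traversable, plus optional road lines with darkened outer segments.
; A vehicle spawner lands on a random side facing across the road and is destroyed with the chunk.
; Inherited helpers then lay a row of landing nodes, attempting a coin before each.
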(event `self.ReceiveBeginPlay`
  (bind _props (`self.Props`))
  (bind (_transformleft _transfrommid _transformright _yposition) (`self.CalculateFloorTransform`))
  (bind _returnvalue (`|SpawnActorFromClass` "/Game/Blueprints/BP_Floor.BP_Floor_C" _transformleft "Undefined" "OverrideRootScale" null 1 false self null))
  (set `self.LeftFloor` _returnvalue)
  (bind _returnvalue_2 (`|SpawnActorFromClass` "/Game/Blueprints/BP_Floor.BP_Floor_C" _transfrommid "Undefined" "OverrideRootScale" null 1 true self null))
  (set `self.CenterFloor` _returnvalue_2)
  (bind _returnvalue_3 (`|SpawnActorFromClass` "/Game/Blueprints/BP_Floor.BP_Floor_C" _transformright "Undefined" "OverrideRootScale" null 1 false self null))
  (set `self.RightFloor` _returnvalue_3)
  (if (`self.HasLines`)
    (bind _returnvalue_4 (- _yposition 100.0))
    (bind _returnvalue_5 (`|SpawnActorFromClass` "/Game/Blueprints/BP_RoadLines.BP_RoadLines_C" (`KismetMathLibrary.MakeTransform` (`KismetMathLibrary.MakeVector` -2000.0 _returnvalue_4)) "Undefined" "OverrideRootScale" null true null))
    (`KismetArrayLibrary.Array_Add` _props _returnvalue_5)
    (bind _returnvalue_6 (`|SpawnActorFromClass` "/Game/Blueprints/BP_RoadLines.BP_RoadLines_C" (`KismetMathLibrary.MakeTransform` (`KismetMathLibrary.MakeVector` 0.0 _returnvalue_4)) "Undefined" "OverrideRootScale" null false null))
    (`KismetArrayLibrary.Array_Add` _props _returnvalue_6)
    (bind _returnvalue_7 (`|SpawnActorFromClass` "/Game/Blueprints/BP_RoadLines.BP_RoadLines_C" (`KismetMathLibrary.MakeTransform` (`KismetMathLibrary.MakeVector` 2000.0 _returnvalue_4)) "Undefined" "OverrideRootScale" null true null))
    (`KismetArrayLibrary.Array_Add` _props _returnvalue_7))
  (`self.ConstructVehicleSpawner` _yposition)
  (`self.ConstructLandingNodes`))

(event `self.ReceiveDestroyed`
  (for _array_element (`self.VehicleSpawners`)
    (`self.K2_DestroyActor` _array_element)))

(fn `ConstructLandingNodes`
  (set `self.CurrentZPosForLandingNode` -30.0)
  (for _ (range 9)
    (`self.CreateCoinAttempt`)
    (`self.ConstructLandingNode(FloorChunk)` false)))

(fn `ConstructVehicleSpawner`
  (params (PositionY :type "Float (double-precision)"))
  (locals (PositionX :type "Float (double-precision)") (FacingLeft :type Boolean))
  (bind _output_get (set `local.FacingLeft` (`KismetMathLibrary.RandomBool`)))
  (if _output_get
    (set `local.PositionX` 2800.0)
    (else
      (bind _output_get_2 (set `local.PositionX` -2800.0))))
  (bind _returnvalue (`|SpawnActorFromClass` "/Game/Blueprints/BP_VehicleSpawner.BP_VehicleSpawner_C" (`KismetMathLibrary.MakeTransform` (`KismetMathLibrary.MakeVector` _output_get_2 PositionY -10.0)) "Undefined" "OverrideRootScale" null _output_get (`self.ChickenRef`) null))
  (`KismetArrayLibrary.Array_Add` (`self.VehicleSpawners`) _returnvalue))

(fn `UserConstructionScript`
  (`parent.UserConstructionScript`))