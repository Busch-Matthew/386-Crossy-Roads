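; Water row floor chunk for a lane-crossing game, offering floating logs, lilypads or both as crossings.
; BeginPlay spawns three floor sections and landing nodes, adding up to three lilypads at distinct clear columns.
; Logs prefill the row, then spawn off one side on a timer, spaced by the previous log's random length and the row's random speed bonus.
; Tick also checks for chunk removal, and destroying the chunk destroys its lilypads.
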(event `self.ReceiveBeginPlay`
  (bind (_transformleft _transfrommid _transformright) (`self.CalculateFloorTransform`))
  (bind _returnvalue (`|SpawnActorFromClass` "/Game/Blueprints/BP_Floor.BP_Floor_C" _transformleft "Undefined" "OverrideRootScale" null 2 false self null))
  (set `self.LeftFloor` _returnvalue)
  (bind _returnvalue_2 (`|SpawnActorFromClass` "/Game/Blueprints/BP_Floor.BP_Floor_C" _transfrommid "Undefined" "OverrideRootScale" null 2 true self null))
  (set `self.CenterFloor` _returnvalue_2)
  (bind _returnvalue_3 (`|SpawnActorFromClass` "/Game/Blueprints/BP_Floor.BP_Floor_C" _transformright "Undefined" "OverrideRootScale" null 2 false self null))
  (set `self.RightFloor` _returnvalue_3)
  (`self.ConstructLandingNodes`)
  (if (`self.CreateLogs`)
    (`self.ConstructInitialLogs`)))

(event `self.ReceiveTick`
  (params (DeltaSeconds :type "Float (single-precision)"))
  (if (`self.CreateLogs`)
    (`self.ConstructLogAttempt` DeltaSeconds))
  (`self.CheckIfDestroyFloorChunk`))

(event `self.ReceiveDestroyed`
  (for _array_element (`self.Lilypads`)
    (`self.K2_DestroyActor` _array_element)))

(fn `AddExtraLogSpeedRand`
  (set `self.ExtraLogSpeedCenter` (`KismetMathLibrary.RandomFloatInRange` 0.0 200.0)))

(fn `CalculateLogCreationOffsetNext`
  (returns (`RandomX Pos` :type "Float (double-precision)"))
  (`/Engine/EditorBlueprintResources/StandardMacros.IsValid` (`self.CurrentLogCreated`)
    (:`Is Valid`
      (switch `int` (`/Game/Blueprints/BP_Log.Length` (`self.CurrentLogCreated`))
        (:`1`
          (return (`KismetMathLibrary.RandomFloatInRange` 400.0 500.0)))
        (:`2`
          (return (`KismetMathLibrary.RandomFloatInRange` 600.0 700.0)))
        (:`3`
          (return (`KismetMathLibrary.RandomFloatInRange` 800.0 900.0)))))
    (:`Is Not Valid`
      (return (`KismetMathLibrary.RandomFloatInRange` 0.0 100.0)))))

(fn `ConstructInitialLogs`
  (locals (`LogCreateX Pos` :type "Float (double-precision)"))
  (if (`self.CreateLogsLeft`)
    (set `local.LogCreateX Pos` -900.0)
    (while (< (`local.LogCreateX Pos`) 900.0)
      (bind _randomx_pos (`self.CalculateLogCreationOffsetNext`))
      (bind _output_get (set `local.LogCreateX Pos` (+ _randomx_pos (`local.LogCreateX Pos`))))
      (`self.ConstructLog` _output_get))
    (else
      (set `local.LogCreateX Pos` 900.0)
      (while (> (`local.LogCreateX Pos`) -900.0)
        (bind _randomx_pos_2 (`self.CalculateLogCreationOffsetNext`))
        (bind _output_get_2 (set `local.LogCreateX Pos` (- (`local.LogCreateX Pos`) _randomx_pos_2)))
        (`self.ConstructLog` _output_get_2)))))

(fn `ConstructLandingNodes`
  (set `self.CurrentZPosForLandingNode` -60.0)
  (for _ (range 9)
    (`self.ConstructLandingNode(FloorChunk)` true))
  (if (`self.CreateLilypads`)
    (`self.ConstructLilypadsMultiple`)))

(fn `ConstructLilypad`
  (params (CurrentX :type "Float (double-precision)"))
  (bind (_returnvalue_x _returnvalue_y _returnvalue_z) (`KismetMathLibrary.BreakVector` (`self.K2_GetActorLocation`)))
  (if (not (== CurrentX -1.0))
    (bind _returnvalue (`|SpawnActorFromClass` "/Game/Blueprints/BP_Lilypads.BP_Lilypads_C" (`KismetMathLibrary.MakeTransform` (`KismetMathLibrary.MakeVector` CurrentX _returnvalue_y (- _returnvalue_z 30.0))) "Undefined" "OverrideRootScale" null null))
    (`KismetArrayLibrary.Array_Add` (`self.Lilypads`) _returnvalue)))

(fn `ConstructLilypadsMultiple`
  (bind _currentclearcolumnposx3 (`self.CurrentClearColumnPosX3`))
  (if (>= (`self.NumberLilypadsToCreate`) 1)
    (`self.ConstructLilypad` (`self.CurrentClearColumnPosX1`))
    (if (>= (`self.NumberLilypadsToCreate`) 2)
      (if (not (== (`self.CurrentClearColumnPosX1`) (`self.CurrentClearColumnPosX2`)))
        (`self.ConstructLilypad` (`self.CurrentClearColumnPosX2`))
        (if (>= (`self.NumberLilypadsToCreate`) 3)
          (if (not (or (== (`self.CurrentClearColumnPosX2`) _currentclearcolumnposx3) (== _currentclearcolumnposx3 (`self.CurrentClearColumnPosX1`))))
            (`self.ConstructLilypad` (`self.CurrentClearColumnPosX3`))))))))

(fn `ConstructLog`
  (params (LocationX :type "Float (double-precision)"))
  (returns (ReturnLog :type "/Game/Blueprints/BP_Log Object Reference"))
  (bind (_returnvalue_x _returnvalue_y _returnvalue_z) (`KismetMathLibrary.BreakVector` (`self.K2_GetActorLocation`)))
  (bind _returnvalue (`|SpawnActorFromClass` "/Game/Blueprints/BP_Log.BP_Log_C" (`KismetMathLibrary.MakeTransform` (`KismetMathLibrary.MakeVector` LocationX _returnvalue_y _returnvalue_z)) "Undefined" "OverrideRootScale" null (`KismetMathLibrary.RandomIntegerInRange` 1 3) (not (`self.CreateLogsLeft`)) (`self.ExtraLogSpeedCenter`) null))
  (bind _output_get (set `self.CurrentLogCreated` _returnvalue))
  (return _output_get))

(fn `ConstructLogAttempt`
  (params (DeltaTime :type "Float (double-precision)"))
  (bind _returnvalue (/ (`self.ExtraLogSpeedCenter`) 400.0))
  (bind _output_get (set `self.CurrentCreateLogTime` (+ DeltaTime (`self.CurrentCreateLogTime`))))
  (if (>= _output_get (`self.MaxCreateLogTime`))
    (if (`self.CreateLogsLeft`)
      (`self.ConstructLog` -2800.0)
      (else
        (`self.ConstructLog` 2800.0)))
    (set `self.CurrentCreateLogTime` 0.0)
    (switch `int` (`/Game/Blueprints/BP_Log.Length` (`self.CurrentLogCreated`))
      (:`1`
        (set `self.MaxCreateLogTime` (- (`KismetMathLibrary.RandomFloatInRange` 1.25 1.5) _returnvalue)))
      (:`2`
        (set `self.MaxCreateLogTime` (- (`KismetMathLibrary.RandomFloatInRange` 1.5 1.75) _returnvalue)))
      (:`3`
        (set `self.MaxCreateLogTime` (- (`KismetMathLibrary.RandomFloatInRange` 2.0 2.25) _returnvalue))))))

(fn `UserConstructionScript`
  (if (`self.CreateLogs`)
    (set `self.MaxCreateLogTime` (`KismetMathLibrary.RandomFloatInRange` 0.0 1.0))
    (`self.AddExtraLogSpeedRand`)))