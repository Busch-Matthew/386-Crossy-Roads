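; Game mode for a Crossy Road-style game that creates the UI, sets the camera, procedurally builds lanes and reloads the Gameplay level after game over.
; ConstructFloors fills up to 20 lanes past the player with grass, road, water and railroad chunks, avoiding consecutive repeats.
; Random chunk lengths depend on forward progress.
; Shared clear-column positions feed grass and water lanes, with rules limiting same-direction log rows and spacing out lilypads.
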(event `self.ReceiveBeginPlay`
  (bind _returnvalue (`GameplayStatics.GetPlayerController` 0))
  (`self.CreateUI`)
  (`self.EnableInput` _returnvalue null)
  (set `PlayerController.bShowMouseCursor` true _returnvalue)
  (set `self.CanRunProgram` true)
  (bind _outactors (`GameplayStatics.GetAllActorsWithTag` "Camera"))
  (for _array_element _outactors
    (bind _asbp_main_camera (cast `/Game/Blueprints/BP_MainCamera` _array_element))
    (bind _output_get (set `self.CameraRef` _asbp_main_camera))
    (`PlayerController.SetViewTargetWithBlend` (`GameplayStatics.GetPlayerController` 0) _output_get 0.0 "VTBlend_Linear" 0.0 false)))

(event `self.ReceiveTick`
  (params (DeltaSeconds :type "Float (single-precision)"))
  (if (`self.CanRunProgram`)
    (if (`self.ConstructedInitialFloorChunks`)
      (if (`self.IsGameOver`)
        (`KismetSystemLibrary.Delay` 3.0)
        (`GameplayStatics.OpenLevel` "Gameplay"))
      (else
        (`self.ConstructInitFloors`)
        (set `self.ConstructedInitialFloorChunks` true)))))

(fn `CalcCurrentFloorTypeCreate`
  (set `self.PreviousFloorTypeCreated` (`self.CurrentFloorTypeCreated`))
  (set `self.CurrentFloorTypeCreated` (`KismetMathLibrary.RandomInteger` 4))
  (if (== (`self.CurrentFloorTypeCreated`) (`self.PreviousFloorTypeCreated`))
    (switch `int` (`self.PreviousFloorTypeCreated`)
      (:`0`
        (set `self.CurrentFloorTypeCreated` 1))
      (:`1`
        (set `self.CurrentFloorTypeCreated` 2))
      (:`2`
        (set `self.CurrentFloorTypeCreated` 3))
      (:`3`
        (set `self.CurrentFloorTypeCreated` 0)))))

(fn `CalcFloorSpawnY`
  (returns (`Position Y` :type "Float (double-precision)"))
  (return (- (* (`self.FloorSpawnYDelta`) (`KismetMathLibrary.Conv_IntToDouble` (`self.CurrentFloorIndex`))) 200.0)))

(fn `ConstructFloors`
  (bind _returnvalue (+ (`KismetMathLibrary.RandomInteger` (- 6 (/ (`self.NumChunksExploredFrwrd`) 20))) 1))
  (bind _returnvalue_2 (+ (`KismetMathLibrary.RandomInteger` (- 6 (/ (`self.NumChunksExploredFrwrd`) 20))) 1))
  (while (< (- (`self.CurrentFloorIndex`) (`self.PlayerPositionIndex`)) 20)
    (`self.CalcCurrentFloorTypeCreate`)
    (switch `int` (`self.CurrentFloorTypeCreated`)
      (:`0`
        (if (< _returnvalue_2 1)
          (`self.CreateGrassFloorChunk` _returnvalue_2)
          (else
            (`self.CreateGrassFloorChunk` 1))))
      (:`1`
        (`self.CreateRoadFloorChunk` _returnvalue))
      (:`2`
        (set `self.CreatedLilypadsWaterChunkGroupStarted` false)
        (`self.CreateWaterFloorChunk` _returnvalue))
      (:`3`
        (`self.CreateRailroadFloorChunk` _returnvalue)))))

(fn `ConstructInitFloors`
  (`self.CreateGrassFloorChunk` 8)
  (`self.CreateGrassFloorChunk` 2 true)
  (`self.ConstructFloors`))

(fn `CountNumLilypadsCreate`
  (set `self.NumLilypadsCreate` 0)
  ;[1 1 1] Clear Column Pos X1
  (if (!= (`self.ClearColPosX1`) -1.0)
    (set `self.NumLilypadsCreate` (+ (`self.NumLilypadsCreate`) 1)))
  ;[1 1 1] Clear Column Pos X2
  (if (!= (`self.ClearColPosX2`) -1.0)
    (set `self.NumLilypadsCreate` (+ (`self.NumLilypadsCreate`) 1))
    ;[1 1 1] Clear Column Pos X3
    (if (!= (`self.ClearColPosx3`) -1.0)
      (set `self.NumLilypadsCreate` (+ (`self.NumLilypadsCreate`) 1)))))

(fn `CreateClearColPos`
  (bind _returnvalue (- (* (`KismetMathLibrary.RandomInteger` 8) 200.0) 800.0))
  (set `self.ClearColPosX1` -1.0)
  (set `self.ClearColPosX2` -1.0)
  (set `self.ClearColPosx3` -1.0)
  (for _index (range (+ (`KismetMathLibrary.RandomInteger` 2) 1))
    (switch `int` _index
      (:`0`
        (set `self.ClearColPosX1` _returnvalue))
      (:`1`
        (set `self.ClearColPosX2` _returnvalue))
      (:`2`
        (set `self.ClearColPosx3` _returnvalue)))))

(fn `CreateGrassFloorChunk`
  (params (NumFloors :type Integer) (CenterClearCol :type Boolean))
  (if (not (== (`self.PreviousFloorTypeCreated`) 2))
    (`self.CreateClearColPos`))
  (if CenterClearCol
    (set `self.ClearColPosx3` 0.0))
  (for _index (range NumFloors)
    (set `self.CurrentFloorIndex` (+ (`self.CurrentFloorIndex`) 1))
    (bind _position_y (`self.CalcFloorSpawnY`))
    (`|SpawnActorFromClass` "/Game/Blueprints/BP_Grass.BP_Grass_C" (`KismetMathLibrary.MakeTransform` (`KismetMathLibrary.MakeVector` 0.0 _position_y)) "Undefined" "OverrideRootScale" null (not (== (mod _index 2) 0)) (`self.ClearColPosX1`) (`self.ClearColPosX2`) (`self.ClearColPosx3`) (`self.ChickenRef`) _position_y null)))

(fn `CreateRailroadFloorChunk`
  (params (NumFloors :type Integer))
  (for _ (range NumFloors)
    (set `self.CurrentFloorIndex` (+ (`self.CurrentFloorIndex`) 1))
    (bind _position_y (`self.CalcFloorSpawnY`))
    (`|SpawnActorFromClass` "/Game/Blueprints/BP_Railroad.BP_Railroad_C" (`KismetMathLibrary.MakeTransform` (`KismetMathLibrary.MakeVector` 0.0 _position_y)) "Undefined" "OverrideRootScale" null (`self.ChickenRef`) _position_y null)))

(fn `CreateRoadFloorChunk`
  (params (NumFloors :type Integer))
  (for _index (range NumFloors)
    (set `self.CurrentFloorIndex` (+ (`self.CurrentFloorIndex`) 1))
    (bind _position_y (`self.CalcFloorSpawnY`))
    (`|SpawnActorFromClass` "/Game/Blueprints/BP_Road.BP_Road_C" (`KismetMathLibrary.MakeTransform` (`KismetMathLibrary.MakeVector` 0.0 _position_y)) "Undefined" "OverrideRootScale" null (>= _index 1) (`self.ChickenRef`) _position_y null)))

(fn `CreateUI`
  (bind _returnvalue (`|CreateWidget` "/Game/UI/UI_GAMEPLAY.UI_GAMEPLAY_C"))
  (set `/Game/UI/UI_GAMEPLAY.Game Mode REF` self _returnvalue)
  (`UserWidget.AddToViewport` _returnvalue 0))

(fn `CreateWaterFloorChunk`
  (params (NumFloors :type Integer))
  (for _ (range NumFloors)
    (set `self.CurrentFloorIndex` (+ (`self.CurrentFloorIndex`) 1))
    (bind _position_y (`self.CalcFloorSpawnY`))
    (if (== (`KismetMathLibrary.RandomIntegerInRange` 0 4) 0)
      (if (`self.CanCreateLilyads`)
        ;[1 1 1] Can Create Lilypads
        (if (`self.CreatedLilypadsWaterChunkGroupStarted`)
          (`self.CreateClearColPos`))
        (`self.CountNumLilypadsCreate`)
        (bind _returnvalue (`KismetMathLibrary.MakeTransform` (`KismetMathLibrary.MakeVector` 0.0 _position_y)))
        (`|SpawnActorFromClass` "/Game/Blueprints/BP_Water.BP_Water_C" _returnvalue "Undefined" "OverrideRootScale" null false false true (`self.NumLilypadsCreate`) (`self.ClearColPosX1`) (`self.ClearColPosX2`) (`self.ClearColPosx3`) (`self.ChickenRef`) _position_y null)
        (set `self.CreatedLilypadsWaterChunkGroupStarted` true)
        (set `self.CanCreateLilyads` false)
        (set `self.CreatedLeftLogsSinceLilypads` false)
        (set `self.CreatedRightLogsSinceLilypadds` false)
        (else
          ;[1 1 1] Can't Create Lilypads; Can Create Logs
          (bind _output_get (set `self.CreateLogsLeft` (`KismetMathLibrary.RandomBool`) :!label _label))
          (if (== _output_get (`self.PreviousLogCreationDirection`))
            (bind _output_get_2 (set `self.NumLogsCreatedSameDir` (+ (`self.NumLogsCreatedSameDir`) 1)))
            (if (> _output_get_2 2)
              (bind _output_get_3 (set `self.CreateLogsLeft` (not (`self.CreateLogsLeft`))))
              (set `self.NumLogsCreatedSameDir` 1)
              (set `self.PreviousLogCreationDirection` _output_get_3))
            (else
              (set `self.NumLogsCreatedSameDir` 1)))
          (`|SpawnActorFromClass` "/Game/Blueprints/BP_Water.BP_Water_C" _returnvalue "Undefined" "OverrideRootScale" null true (`self.CreateLogsLeft`) false 0 (`self.ClearColPosX1`) (`self.ClearColPosX2`) (`self.ClearColPosx3`) (`self.ChickenRef`) _position_y null)
          (if (`self.CreateLogsLeft`)
            (set `self.CreatedLeftLogsSinceLilypads` true)
            (else
              (set `self.CreatedRightLogsSinceLilypadds` true)))
          (if (`self.CreatedLeftLogsSinceLilypads`)
            (if (`self.CreatedRightLogsSinceLilypadds`)
              (set `self.CanCreateLilyads` true)))
          (set `self.PreviousLogCreationDirection` (`self.CreateLogsLeft`))))
      (else
        (goto _label)))))

(fn `UserConstructionScript`)