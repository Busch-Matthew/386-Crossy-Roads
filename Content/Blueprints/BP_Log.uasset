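; Moving log actor that travels along the X axis and can be jumped on, with three length variants.
; BeginPlay picks the mesh and box X scale from Length.
; Each Tick moves it by a zone-based center or side speed plus a random extra, signed by direction, and destroys it beyond the outer X bounds.
; Tick also plays a random jump-on sound when landed on and calls a bouncing animation.
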(event `self.ReceiveBeginPlay`
  (bind _staticmesh (`self.StaticMesh`))
  (`parent.ReceiveBeginPlay`)
  (switch `int` (`self.Length`)
    (:`1`
      (set `self.ScaleX` 1.75)
      (`StaticMeshComponent.SetStaticMesh` _staticmesh "/Game/media/meshes/log3.log3"))
    (:`2`
      (set `self.ScaleX` 5.0)
      (`StaticMeshComponent.SetStaticMesh` _staticmesh "/Game/media/meshes/log2.log2"))
    (:`3`
      (set `self.ScaleX` 8.5)
      (`StaticMeshComponent.SetStaticMesh` _staticmesh "/Game/media/meshes/log1.log1")))
  (`SceneComponent.SetRelativeScale3D` (`self.Box`) (`KismetMathLibrary.MakeVector` (`self.ScaleX`))))

(event `self.ReceiveTick`
  (params (DeltaSeconds :type "Float (single-precision)"))
  (`self.MoveLog` DeltaSeconds)
  (`self.CheckLogOutOfBounds`)
  (`self.AttemptPlayJumpOnSound`)
  (`self.BouncingAnimation` DeltaSeconds))

(fn `AttemptPlayJumpOnSound`
  (bind _returnvalue (`KismetMathLibrary.RandomFloatInRange` 0.5 1.0))
  (if (and (== (`self.CurrentJumpOnTime`) 0.0) (`self.IsBeingJumpedOn`))
    (if (`KismetMathLibrary.RandomBool`)
      (`GameplayStatics.PlaySound2D` "/Game/media/sounds/log1.log1" _returnvalue 1.0 0.0 null null)
      (else
        (`GameplayStatics.PlaySound2D` "/Game/media/sounds/log2.log2" _returnvalue 1.0 0.0 null null)))))

(fn `CheckLogOutOfBounds`
  (bind _returnvalue_x (`KismetMathLibrary.BreakVector` (`self.K2_GetActorLocation`)))
  (if (> _returnvalue_x 2800.0)
    (`self.K2_DestroyActor` :!label _label)
    (elif (< _returnvalue_x -2800.0)
      (goto _label))))

(fn `MoveLog`
  (params (DeltaTime :type "Float (double-precision)"))
  (bind _returnvalue_x (`KismetMathLibrary.BreakVector` (`self.K2_GetActorLocation`)))
  (if (`self.MoveLeft`)
    (set `self.FloatInverse` -1.0))
  (if (>= _returnvalue_x -1400.0)
    (if (<= _returnvalue_x 1400.0)
      (set `self.CurrentSpeed` (`self.MoveSpeedCenter`))
      (else
        (set `self.CurrentSpeed` (`self.MoveSpeedLeftRight`) :!label _label)))
    (else
      (goto _label)))
  (bind _output_get (set `self.CurrentSpeed` (* (`self.FloatInverse`) (+ (`self.CurrentSpeed`) (`self.ExtraMoveSpeedRand`)))))
  (`self.K2_AddActorWorldOffset` (`KismetMathLibrary.MakeVector` (* _output_get DeltaTime))))

(fn `UserConstructionScript`
  (`parent.UserConstructionScript`))