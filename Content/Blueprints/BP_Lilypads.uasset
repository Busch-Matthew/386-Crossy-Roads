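; Lilypad actor that bounces when jumped on and spins while a character stands on it.
; On BeginPlay it picks a random rotation rate and runs a random switch leading to a BP_Coin spawn at its location.
; Each Tick plays the lily pad sound at the start of a jump-on, runs BouncingAnimation, and applies the frame-time-scaled spin while HasChxOnTop is set.
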(event `self.ReceiveBeginPlay`
  (`parent.ReceiveBeginPlay`)
  (set `self.Rotation` (`KismetMathLibrary.MakeRotator` 0.0 0.0 (`KismetMathLibrary.RandomFloatInRange` -20.0 20.0)))
  (switch `int` (`KismetMathLibrary.RandomInteger` 3)
    (:`0`
      _)
    (:`1`
      _))
  (`|SpawnActorFromClass` "/Game/Blueprints/BP_Coin.BP_Coin_C" (`KismetMathLibrary.MakeTransform` (`self.K2_GetActorLocation`)) "Undefined" "OverrideRootScale" null null))

(event `self.ReceiveTick`
  (params (DeltaSeconds :type "Float (single-precision)"))
  (bind _maindeltasecs (`self.MainDeltaSecs`))
  (set `self.MainDeltaSecs` DeltaSeconds)
  (`self.AttemptPlayJumpOnSound`)
  (`self.BouncingAnimation` _maindeltasecs)
  (if (`self.HasChxOnTop`)
    (`self.K2_AddActorLocalRotation` (* (`self.Rotation`) _maindeltasecs))))

(fn `AttemptPlayJumpOnSound`
  (if (and (== (`self.CurrentJumpOnTime`) 0.0) (`self.IsBeingJumpedOn`))
    (`GameplayStatics.PlaySound2D` "/Game/media/sounds/lily_pad.lily_pad" 1.0 1.0 0.0 null null)))

(fn `UserConstructionScript`
  (`parent.UserConstructionScript`))