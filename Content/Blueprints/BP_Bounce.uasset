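; BP_Bounce is an actor that plays a short vertical bounce animation when flagged as being jumped on.
; While the flag is set, Tick accumulates time and, after a start delay, drives a hard-coded parabolic Z offset from a cached height.
; When the time window ends, it clears the flag, timer and offset, snapping back to that height.
; The flag and cached height are not set within this Blueprint.
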(event `self.ReceiveBeginPlay`
  (set `self.MaxJumpOnTime` (+ (`self.MaxStartJumpTime`) 0.2)))

(event `self.ReceiveTick`
  (params (DeltaSeconds :type "Float (single-precision)"))
  (`self.BouncingAnimation` DeltaSeconds))

(fn `BouncingAnimation`
  (params (DeltaTime :type "Float (double-precision)"))
  (bind (_returnvalue_x _returnvalue_y) (`KismetMathLibrary.BreakVector` (`self.K2_GetActorLocation`)))
  (if (`self.IsBeingJumpedOn`)
    (`self.JumpedOnAnimation` DeltaTime)
    (`self.K2_SetActorLocation` (`KismetMathLibrary.MakeVector` _returnvalue_x _returnvalue_y (+ (`self.CashedZPos`) (`self.JumpedOnZOffset`))))))

(fn `JumpedOnAnimation`
  (params (DeltaTime :type "Float (double-precision)"))
  (set `self.CurrentJumpOnTime` (+ DeltaTime (`self.CurrentJumpOnTime`)))
  (if (>= (`self.CurrentJumpOnTime`) (`self.MaxStartJumpTime`))
    (if (>= (`self.CurrentJumpOnTime`) (`self.MaxJumpOnTime`))
      (`self.ResetAnimation`)
      (else
        (set `self.JumpedOnZOffset` (* (- (`KismetMathLibrary.Square` (- (* (- (`self.CurrentJumpOnTime`) 0.1) 8.0) 1.0)) 1.0) 20.0))))))

(fn `ResetAnimation`
  (set `self.IsBeingJumpedOn` false)
  (set `self.JumpedOnZOffset` 0.0)
  (set `self.CurrentJumpOnTime` 0.0))

(fn `UserConstructionScript`)