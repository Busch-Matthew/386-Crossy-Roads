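; Main camera actor that follows the player's BP_Chicken along the Y axis.
; BeginPlay caches the player pawn as ChickenRef if the cast succeeds.
; Tick moves the camera to the chicken's Y plus OffsetY, holding X and height fixed.
; BeginPlay also clears GamemodeRef, then writes this camera into that empty reference's ChickenRef, so that assignment has no valid target.
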(event `self.ReceiveBeginPlay`
  (bind _asbp_chicken (cast `/Game/Blueprints/BP_Chicken` (`GameplayStatics.GetPlayerPawn` 0)))
  (set `self.ChickenRef` _asbp_chicken)
  (bind _output_get (set `self.GamemodeRef` null))
  (set `/Game/Blueprints/BP_GameModeCrossyRoads.ChickenRef` self _output_get))

(event `self.ReceiveTick`
  (params (DeltaSeconds :type "Float (single-precision)"))
  (`self.K2_SetActorLocation` (`KismetMathLibrary.MakeVector` 0.0 (+ (.y (`self.K2_GetActorLocation` (`self.ChickenRef`))) (`self.OffsetY`)) 1300.0)))

(fn `UserConstructionScript`)